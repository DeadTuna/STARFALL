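; Pinball is a pickup weapon that auto-fires Bullet actors from the player toward the mouse cursor.
; Overlap shows a PressE prompt; Interact assigns it to the character's Weapon, briefly animates its scale, then hides it.
; The pinball event toggles firing, looping on a short cooldown while enabled.
; SpawnProjectile derives spawn offset and rotation from the screen-space direction between player and cursor, applied as world yaw.
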(event `pinball`
  (params (toggle :type Boolean))
  (bind _output_get (set `self.can fire` toggle))
  (if _output_get
    (if (and (`self.can fire`) (not (`self.fire delay`))) :!label _label
      (set `self.fire delay` true)
      (`self.spawn projectile`)
      (`KismetSystemLibrary.Delay` 0.2)
      (set `self.fire delay` false)
      (goto _label))))

(event `self.ReceiveActorBeginOverlap`
  (params (OtherActor :type "Actor Object Reference"))
  (cast `/Game/Character/MyCharacter` OtherActor)
  (bind _returnvalue (`|CreateWidget` "/Game/UI/pressE.pressE_C" (`GameplayStatics.GetPlayerController` 0)))
  (`UserWidget.AddToViewport` _returnvalue 0))

(event `self.ReceiveActorEndOverlap`
  (params (OtherActor :type "Actor Object Reference"))
  (`Widget.RemoveFromParent` (stale `self.ReceiveActorBeginOverlap` _returnvalue)))

(event `/Game/Blueprints/interfaces/interactable.Interact`
  (params (Interactable :type "Actor Object Reference"))
  (bind _asmy_character (cast `/Game/Character/MyCharacter` Interactable))
  (set `/Game/Character/MyCharacter.weapon` self _asmy_character)
  (`self.SetActorScale3D` (+ (`self.GetActorScale3D` Interactable) (-0.3 -0.7 0.0)))
  (`KismetSystemLibrary.Delay` 0.02)
  (`self.SetActorScale3D` (+ (`self.GetActorScale3D` Interactable) (-0.3 -0.3 0.0)))
  (`KismetSystemLibrary.Delay` 0.02)
  (`self.SetActorScale3D` (/ (`self.GetActorScale3D` Interactable) 1.2))
  (`self.SetActorHiddenInGame` true)
  (`self.SetActorEnableCollision` false))

(fn `spawn projectile`
  (bind _returnvalue (`GameplayStatics.GetPlayerController` 0))
  (bind _returnvalue_2 (`GameplayStatics.GetPlayerCharacter` 0))
  (bind (_locationx _locationy) (`PlayerController.GetMousePosition` _returnvalue))
  (bind _returnvalue_3 (`KismetMathLibrary.FindLookAtRotation` (`KismetMathLibrary.Conv_Vector2DToVector` (`PlayerController.ProjectWorldLocationToScreen` _returnvalue (`self.K2_GetActorLocation` _returnvalue_2) false)) (`KismetMathLibrary.MakeVector` _locationx _locationy)))
  (`|SpawnActorFromClass` "/Game/Blueprints/Weapon/bullet.bullet_C" (`KismetMathLibrary.MakeTransform` (+ (`self.K2_GetActorLocation` _returnvalue_2) (`KismetMathLibrary.GreaterGreater_VectorRotator` (100.0 0.0 0.0) _returnvalue_3)) _returnvalue_3 (.scale (`self.GetTransform` (`GameplayStatics.GetPlayerCharacter` 0)))) "Undefined" "OverrideRootScale" null null))

(fn `UserConstructionScript`)