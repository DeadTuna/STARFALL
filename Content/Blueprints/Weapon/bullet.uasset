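; Bouncing projectile Blueprint for a weapon bullet that restarts the level when it hits the player character.
; All logic runs on the ProjectileMovement bounce event, which plays a bounce sound and counts impacts, destroying the actor on the fourth.
; If the hit actor is MyCharacter, it plays a death camera shake, then reopens the current level after a short delay.
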(event `self.ProjectileMovement.OnProjectileBounce`
  (params (ImpactResult :type "HitResult Structure (by ref)") (ImpactVelocity :type "Vector Structure (by ref)"))
  (bind (_bblockinghit _binitialoverlap _time _distance _location _impactpoint _normal _impactnormal _physmat _hitactor) (`GameplayStatics.BreakHitResult` ImpactResult))
  (`GameplayStatics.PlaySoundAtLocation` "/Game/Music/bounce__online-audio-converter_com_.bounce__online-audio-converter_com_" _location (struct) 1.0 1.0 0.0 null null null)
  (set `self.Bounce` (+ (`self.Bounce`) 1.0))
  (if (>= (`self.Bounce`) 4.0)
    (`self.K2_DestroyActor`))
  (cast `/Game/Character/MyCharacter` _hitactor)
  (`GameplayStatics.PlayWorldCameraShake` "/Game/Blueprints/camera/DeathShake.DeathShake_C" (`self.K2_GetActorLocation` _hitactor) 5000.0 5000.0 1.0 true)
  (`KismetSystemLibrary.Delay` 0.2)
  (bind _returnvalue (`GameplayStatics.GetCurrentLevelName` true))
  (`GameplayStatics.OpenLevel` (`KismetStringLibrary.Conv_StringToName` _returnvalue)))

(fn `UserConstructionScript`)